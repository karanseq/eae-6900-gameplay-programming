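; BP_GateDestructible is a destructible gate made of five cube meshes that disappear as it takes damage.
; The construction script stores the cubes in an ordered Meshes array.
; On AnyDamage, it hides the mesh at index HitsTaken minus one and sets that mesh to NoCollision.
; HitsTaken is only read here; this graph does not increment it.
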(event `self.ReceiveBeginPlay`)

(event `self.ReceiveAnyDamage`
  (params (Damage :type "Float (single-precision)") (DamageType :type "DamageType Object Reference") (InstigatedBy :type "Controller Object Reference") (DamageCauser :type "Actor Object Reference"))
  (bind _output (`|GetArrayItem` (`self.Meshes`) (- (`self.HitsTaken`) 1)))
  (`PrimitiveComponent.SetCollisionProfileName` _output "NoCollision")
  (`SceneComponent.SetVisibility` _output false false))

(fn `UserConstructionScript`
  (set `self.Meshes` (`|MakeArray` (`self.Cube4`) (`self.Cube1`) (`self.Cube3`) (`self.Cube2`) (`self.Cube`))))