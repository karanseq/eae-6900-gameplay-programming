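; BP_TowerSpawner is a tower spawn point that carries a world-space widget for choosing a physical, magical or slowing tower.
; On BeginPlay it binds handlers to the three W_TowerSelect buttons, though their logic is not shown, and ShowTowerSelection makes the widget visible.
; It tracks the current camera through BP_TDPlayerController's camera-toggle event and rotates the widget to face that camera every Tick.
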(event `self.ReceiveBeginPlay`
  ;[1 1 1] Camera
  (bind _asbp_tdplayer_controller (cast `/Game/Blueprints/Shared/BP_TDPlayerController` (`GameplayStatics.GetPlayerController` 0)))
  (add `/Game/Blueprints/Shared/BP_TDPlayerController.OnCameraToggled` _asbp_tdplayer_controller (`|CreateDelegate` :!event `OnCameraToggled`))
  (set `self.CurrentCamera` (`/Game/Blueprints/Shared/BP_TDPlayerController.GetCurrentCamera` _asbp_tdplayer_controller))
  ;[1 1 1] UI
  (bind _asw_tower_select (cast `/Game/Blueprints/UI/W_TowerSelect` (`WidgetComponent.GetUserWidgetObject` (`self.Widget`))))
  (add `Button.OnClicked` (`/Game/Blueprints/UI/W_TowerSelect.Button_Physical` _asw_tower_select) (`|CreateDelegate` :!event `OnPhysicalTowerSelected`))
  (add `Button.OnClicked` (`/Game/Blueprints/UI/W_TowerSelect.Button_Magical` _asw_tower_select) (`|CreateDelegate` :!event `OnMagicalTowerSelected`))
  (add `Button.OnClicked` (`/Game/Blueprints/UI/W_TowerSelect.Button_Slowing` _asw_tower_select) (`|CreateDelegate` :!event `OnSlowingTowerSelected`)))

(event `OnCameraToggled`
  (params (CurrentCamera :type "CameraActor Object Reference"))
  ;[1 1 1] Camera
  (set `self.CurrentCamera` CurrentCamera))

(event `self.ShowTowerSelection`
  ;[1 1 1] UI
  (`SceneComponent.SetVisibility` (`self.Widget`) true false))

(event `self.ReceiveTick`
  (params (DeltaSeconds :type "Float (single-precision)"))
  ;[1 1 1] Camera | UI
  (`SceneComponent.K2_SetWorldRotation` (`self.Widget`) (`KismetMathLibrary.FindLookAtRotation` (`self.K2_GetActorLocation`) (`self.K2_GetActorLocation` (`self.CurrentCamera`))) false false))

(fn `UserConstructionScript`)