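; BP_EnemySpawner relays enemy lifecycle events to the player's on-screen or stored event log.
; On BeginPlay it casts player controller 0 to BP_TDPlayerController and caches its EventLog.
; Spawn, kill and progress-to-base events each build a message from the enemy name and post it in an event-specific color.
; The Blueprint graphs contain only this logging, with no spawning logic and an empty construction script.
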(event `self.ReceiveBeginPlay`
  (bind _asbp_tdplayer_controller (cast `/Game/Blueprints/Shared/BP_TDPlayerController` (`GameplayStatics.GetPlayerController` 0)))
  (set `self.EventLog` (`/Game/Blueprints/Shared/BP_TDPlayerController.EventLog` _asbp_tdplayer_controller)))

(event `self.OnEnemySpawned`
  (params (EnemyName :type String))
  (`/Game/Blueprints/UI/UI_EventLog.AddMessageToLog` (`self.EventLog`) (`KismetStringLibrary.Concat_StrStr` EnemyName " spawned") (`self.SpawnedColor`)))

(event `self.OnEnemyKilled`
  (params (EnemyName :type String))
  (`/Game/Blueprints/UI/UI_EventLog.AddMessageToLog` (`self.EventLog`) (`KismetStringLibrary.Concat_StrStr` EnemyName " killed") (`self.KilledColor`)))

(event `self.OnEnemyMadeProgress`
  (params (EnemyName :type String) (Progress :type Integer))
  (`/Game/Blueprints/UI/UI_EventLog.AddMessageToLog` (`self.EventLog`) (`KismetStringLibrary.Concat_StrStr` EnemyName " is " (`KismetStringLibrary.Conv_IntToString` Progress) "% to base") (`self.ProgressColor`)))

(fn `UserConstructionScript`)