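; Player controller that switches the view between two cameras and manages an on-screen event log.
; On BeginPlay it creates the event log widget and adds it to the viewport, and the L key shows or hides it.
; The C key sets the view target to the other camera, flips the active-camera flag and broadcasts OnCameraToggled with the new camera.
; GetCurrentCamera returns the active camera from that flag.
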(event `self.ReceiveBeginPlay`
  ;[1 1 1] Create the event log
  (bind _returnvalue (`|CreateWidget` "/Game/Blueprints/UI/W_EventLog.W_EventLog_C" self))
  (bind _output_get (set `self.EventLog` _returnvalue))
  (`UserWidget.AddToViewport` _output_get 0))

(event `Key|C`
  (params (Key :type "Key Structure"))
  (:`Pressed`
    (bind _ascamera_actor (cast `CameraActor` (`KismetMathLibrary.SelectObject` (`self.Camera_02`) (`self.Camera_01`) (`self.bIsCamera_01`))))
    (`self.SetViewTargetWithBlend` _ascamera_actor)
    (set `self.bIsCamera_01` (not (`self.bIsCamera_01`)))
    (`self.OnCameraToggled` _ascamera_actor)))

(event `Key|L`
  (params (Key :type "Key Structure"))
  (:`Pressed`
    (if (`self.bIsEventLogVisible`)
      (`Widget.SetVisibility` (`self.EventLog`) "Hidden")
      (set `self.bIsEventLogVisible` false)
      (else
        (`Widget.SetVisibility` (`self.EventLog`) "Visible")
        (set `self.bIsEventLogVisible` true)))))

(fn `GetCurrentCamera`
  (returns (CurrentCamera :type "CameraActor Object Reference"))
  (bind _ascamera_actor (cast `CameraActor` (`KismetMathLibrary.SelectObject` (`self.Camera_01`) (`self.Camera_02`) (`self.bIsCamera_01`))))
  (return _ascamera_actor))

(fn `UserConstructionScript`)