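; BP_BasicEnemy is an enemy that carries a widget health bar which turns to face the player's current camera.
; It gets the camera from BP_TDPlayerController at BeginPlay and binds to that controller's camera-toggle event to track changes.
; OnHealthChanged sets the W_EnemyInfo bar to current over max health, while Tick rotates the widget toward the camera.
; Camera updates, bar updates and rotation all stop once the enemy is dying.
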(event `self.ReceiveBeginPlay`
  (bind _asbp_tdplayer_controller (cast `/Game/Blueprints/Shared/BP_TDPlayerController` (`GameplayStatics.GetPlayerController` 0)))
  (add `/Game/Blueprints/Shared/BP_TDPlayerController.OnCameraToggled` _asbp_tdplayer_controller (`|CreateDelegate` :!event `OnCameraToggled`))
  (set `self.CurrentCamera` (`/Game/Blueprints/Shared/BP_TDPlayerController.GetCurrentCamera` _asbp_tdplayer_controller)))

(event `OnCameraToggled`
  (params (CurrentCamera :type "CameraActor Object Reference"))
  (if (not (`self.bIsDying`))
    (set `self.CurrentCamera` CurrentCamera)))

(event `self.OnHealthChanged`
  (if (not (`self.bIsDying`))
    (bind _asw_enemy_info (cast `/Game/Blueprints/UI/W_EnemyInfo` (`WidgetComponent.GetUserWidgetObject` (`self.UI`))))
    (`ProgressBar.SetPercent` (`/Game/Blueprints/UI/W_EnemyInfo.HealthBar` _asw_enemy_info) (/ (`self.CurrentHealth`) (`self.MaxHealth`)))))

(event `self.ReceiveTick`
  (params (DeltaSeconds :type "Float (single-precision)"))
  (if (not (`self.bIsDying`))
    (`SceneComponent.K2_SetWorldRotation` (`self.UI`) (`KismetMathLibrary.FindLookAtRotation` (`self.K2_GetActorLocation`) (`self.K2_GetActorLocation` (`self.CurrentCamera`))) false false)))

(fn `UserConstructionScript`)