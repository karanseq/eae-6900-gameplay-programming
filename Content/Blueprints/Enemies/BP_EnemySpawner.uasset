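; BP_EnemySpawner is a tower-defense enemy spawner actor that starts wave spawning and reports combat and wave activity to the player's event log.
; On BeginPlay it caches the EventLog from BP_TDPlayerController and tells its SpawnerComponent to start from the first wave.
; Handlers for wave start and end, and for enemy damage, blocks and kills, post color-coded messages naming the wave or the enemy and damage type.
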(event `self.ReceiveBeginPlay`
  ;[1 1 1] Begin play
  (bind _asbp_tdplayer_controller (cast `/Game/Blueprints/Shared/BP_TDPlayerController` (`GameplayStatics.GetPlayerController` 0)))
  (set `self.EventLog` (`/Game/Blueprints/Shared/BP_TDPlayerController.EventLog` _asbp_tdplayer_controller))
  (`SpawnerComponent.StartSpawning` (`self.SpawnerComponent`) 0 false))

(event `self.OnEnemyTookDamage`
  (params (EnemyName :type String) (DamageAmount :type "Float (single-precision)") (Type :type "EStatKind Enum" :default "None"))
  ;[1 1 1] Enemy events
  (`/Game/Blueprints/UI/W_EventLog.AddMessageToLog` (`self.EventLog`) (`KismetStringLibrary.Concat_StrStr` EnemyName " took " (`KismetStringLibrary.Conv_DoubleToString` DamageAmount) " " (`|GetEnumeratorNameAsString` Type)) (`self.Yellow`)))

(event `self.OnWaveStarted`
  (params (WaveIndex :type Integer))
  ;[1 1 1] Wave events
  (`/Game/Blueprints/UI/W_EventLog.AddMessageToLog` (`self.EventLog`) (`KismetStringLibrary.Concat_StrStr` "Wave-" (`KismetStringLibrary.Conv_IntToString` WaveIndex) " started") (`self.Red`)))

(event `self.OnEnemyBlockedDamage`
  (params (EnemyName :type String) (DamageAmount :type "Float (single-precision)") (Type :type "EStatKind Enum" :default "None"))
  ;[1 1 1] Enemy events
  (`/Game/Blueprints/UI/W_EventLog.AddMessageToLog` (`self.EventLog`) (`KismetStringLibrary.Concat_StrStr` EnemyName " blocked " (`|GetEnumeratorNameAsString` Type)) (`self.Red`)))

(event `self.OnWaveEnded`
  (params (WaveIndex :type Integer))
  ;[1 1 1] Wave events
  (`/Game/Blueprints/UI/W_EventLog.AddMessageToLog` (`self.EventLog`) (`KismetStringLibrary.Concat_StrStr` "Wave-" (`KismetStringLibrary.Conv_IntToString` WaveIndex) " ended") (`self.Green`)))

(event `self.OnEnemyKilled`
  (params (EnemyName :type String) (Type :type "EStatKind Enum" :default "None"))
  ;[1 1 1] Enemy events
  (`/Game/Blueprints/UI/W_EventLog.AddMessageToLog` (`self.EventLog`) (`KismetStringLibrary.Concat_StrStr` EnemyName " killed " " by " (`|GetEnumeratorNameAsString` Type)) (`self.Green`)))

(fn `UserConstructionScript`)